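; BP_Chair_HJ is a chair product actor that can be positioned on a plane from a screen location.
; Construction applies the mesh and flattened Plate scale from Ref and hides the Plate, but BeginPlay then overrides the mesh with Basic_chair.
; SetChairPosition deprojects the screen point, line-traces along that ray and moves the Scene component to the hit only when it lands on the referenced Plane actor.
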(event EventTick
  (params (DeltaSeconds :type Float%20%28single-precision%29)))

(event EventBeginPlay
  ;[0.15 0.15 0.15 0.5] Heejung
  (Components|StaticMesh|SetStaticMesh (Variables|Default|GetStaticMesh) "/Game/ARCarRacing/Content/Fab/Basic_Chair/basic_chair/StaticMeshes/basic_chair.basic_chair"))

(fn ConstructionScript
  (CallFunction|AssignProductAsset))

(fn AssignProductAsset
  (bind _ref (Variables|Default|GetRef))
  (bind _plate (Variables|/Game/Blueprint/Ref.Ref_C|GetPlate _ref))
  (Components|StaticMesh|SetStaticMesh (Variables|Default|GetStaticMesh) (Variables|/Game/Blueprint/Ref.Ref_C|GetStaticMesh (Variables|Default|GetRef)))
  (Transformation|SetWorldScale3D (Variables|Default|GetPlate) (Math|Vector|MakeVector _plate _plate 0.0))
  (Rendering|SetVisibility (Variables|Default|GetPlate) false false))

(fn SetChairPosition
  (params (Location :type Vector%202D%20Structure))
  (bind _returnvalue (Game|GetPlayerController 0))
  (bind (_worldposition _worlddirection) (Class|GameplayStatics|DeprojectScreentoWorld _returnvalue Location))
  (bind (_outhit _returnvalue_2) (Collision|LineTraceForObjects _worldposition (+ _worldposition (* _worlddirection 1e+03)) (Utilities|Array|MakeArray "ObjectTypeQuery1" "ObjectTypeQuery2" "ObjectTypeQuery3" "ObjectTypeQuery4" "ObjectTypeQuery5" "ObjectTypeQuery6") false 0 "None"))
  (if _returnvalue_2
    (if (== (.HitActor (Collision|BreakHitResult _outhit)) (Variables|Default|GetPlane))
      (Transformation|SetWorldLocation (Variables|Default|GetScene) (.Location (Collision|BreakHitResult _outhit)) false false))))